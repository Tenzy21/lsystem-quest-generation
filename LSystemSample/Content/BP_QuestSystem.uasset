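; Quest system that procedurally generates a quest on BeginPlay and adds it to its active quests.
; An L-system built at construction expands a start axiom using the player context from the game state.
; Each resulting token is looked up in a token-library DataTable and its linked object is loaded synchronously.
; Only experience and money tokens affect the quest, adding rewards with hardcoded amounts; debug prints show the sequence.
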(event `self.ReceiveBeginPlay`
  (bind _result (`LSystem.ProceedGeneration` (`self.LSystem`) (`|MakeArray` "S") 8 (`self.Context`)))
  (`|ExecutionSequence`
    (:`then_0`
      (set `self.Cache` "")
      (for _array_element _result
        (set `self.Cache` (`KismetStringLibrary.Concat_StrStr` (`self.Cache`) " " _array_element)))
      (`KismetSystemLibrary.PrintString` (`self.Cache`) true true (struct :`G` 0.66 :`B` 1.0 :`A` 1.0) 500.0))
    (:`then_1`
      (`self.GenerateQuest` _result))))

(event `GenerateQuest`
  (params (Axiom :type "Array of String"))
  (bind _newquestcache (`self.NewQuestCache`))
  (bind _returnvalue (`|GenericCreateObject` "/Game/BP_QuestBase.BP_QuestBase_C"))
  (set `self.NewQuestCache` _returnvalue)
  (for _array_element Axiom
    (bind _returnvalue_2 (`|GetDataTableRow` "/Game/DT_TokenLibrary.DT_TokenLibrary" (`KismetStringLibrary.Conv_StringToName` _array_element))
      (:`then`
        (bind (_tokenid _linkedobject) (break `LTokenData` _returnvalue_2))
        (`KismetSystemLibrary.PrintString` _tokenid true true (struct :`R` 1.0 :`G` 0.041135 :`A` 1.0) 50.0)
        (bind _returnvalue_3 (`KismetSystemLibrary.LoadAsset_Blocking` _linkedobject))
        (switch `string` _tokenid
          (:`{G_E}`
            (bind _asbp_exp_reward (cast `/Game/Rewards/BP_ExpReward` _returnvalue_3))
            (`/Game/Rewards/BP_ExpReward.SetExpAmount` _asbp_exp_reward 100)
            (`/Game/BP_QuestBase.AddReward` _newquestcache _asbp_exp_reward))
          (:`{G_G}`
            (bind _asbp_money_reward (cast `/Game/Rewards/BP_MoneyReward` _returnvalue_3))
            (`/Game/Rewards/BP_MoneyReward.SetMoneyAmount` _asbp_money_reward 69)
            (`/Game/BP_QuestBase.AddReward` _newquestcache _asbp_money_reward))))))
  (`KismetArrayLibrary.Array_Add` (`self.ActiveQuests`) (`self.NewQuestCache`)))

(fn `UserConstructionScript`
  (bind _returnvalue (`|GenericCreateObject` "/Game/BP_LSystem.BP_LSystem_C"))
  (set `self.LSystem` _returnvalue)
  (bind _asbp_game_state (cast `/Game/BP_GameState` (`GameplayStatics.GetGameState`)))
  (set `self.Context` (`/Game/BP_GameState.PlayerContext` _asbp_game_state)))