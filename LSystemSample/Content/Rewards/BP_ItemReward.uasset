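; BP_ItemReward spawns a random item as a reward near a stored spawn transform.
; SetSpawn saves the transform, and ProceedReward picks a random row name from ItemsDataTable and looks it up in DT_ItemsAssets.
; If the row is found, it always spawns that ItemAsset class slightly raised, with random horizontal scatter, and prints the actor's name.
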(event `SetSpawn`
  (params (Transform :type "Transform Structure"))
  (set `self.SpawnTransform` Transform))

(event `self.ProceedReward`
  (params (GameState :type "/Game/BP_GameState Object Reference"))
  (bind _spawntransform_location (`KismetMathLibrary.BreakTransform` (`self.SpawnTransform`)))
  (bind _returnvalue (- (* (`KismetMathLibrary.RandomFloat`) 200.0) 100.0))
  (bind _outrownames (`DataTableFunctionLibrary.GetDataTableRowNames` (`self.Items DataTable`)))
  (bind _returnvalue_2 (`|GetDataTableRow` "/Game/DT_ItemsAssets.DT_ItemsAssets" (`KismetArrayLibrary.Array_Random` _outrownames))
    (:`then`
      (bind _returnvalue_3 (`|SpawnActorFromClass` (`.ItemAsset_4_9A5132104E813B63F8CFF2A3C58D14E5` (break `/Game/S_Item` _returnvalue_2)) (`KismetMathLibrary.Conv_VectorToTransform` (`KismetMathLibrary.MakeVector` (+ (.x _spawntransform_location) _returnvalue) (+ _returnvalue (.y _spawntransform_location)) (+ (.z _spawntransform_location) 20.0))) "AlwaysSpawn" "OverrideRootScale" null null))
      (`KismetSystemLibrary.PrintString` (`KismetSystemLibrary.GetDisplayName` _returnvalue_3)))))